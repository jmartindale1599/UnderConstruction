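; BP_Burnable supplies fire ignition and spreading logic for BP_Placeable actors.
; SetOnFire checks CanBurn and the placeable's IsOnFire flag, then switches its Niagara component to NS_Fire, activates it and makes it visible.
; StartFire then spreads the fire in a single overlap pass, calling Burn on each overlapping BP_Placeable that is not already on fire.
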(event `Set OnFire`
  (params (SelfRef :type "Actor Object Reference"))
  (if (`self.CanBurn?`)
    (bind _asbp_placeable (cast `/Game/Placeables/BP_Placeable` SelfRef))
    (if (not (`/Game/Placeables/BP_Placeable.IsOnFire?` _asbp_placeable))
      (bind _niagara (`/Game/Placeables/BP_Placeable.Niagara` _asbp_placeable))
      (`NiagaraComponent.SetAsset` _niagara "/Game/Particles/NS_Fire.NS_Fire" false)
      (`self.Activate` _niagara false)
      (if (not (`SceneComponent.IsVisible` _niagara))
        (`SceneComponent.SetVisibility` _niagara true false))
      (`self.StartFire` null _asbp_placeable))))

(fn `StartFire`
  (params (NiagraParticles :type "NiagaraComponent Object Reference") (SelfRef :type "Actor Object Reference"))
  (`NiagaraComponent.SetAsset` NiagraParticles "/Game/Particles/NS_Fire.NS_Fire" false)
  (for _array_element (`Actor.GetOverlappingActors` SelfRef "/Game/Placeables/BP_Placeable.BP_Placeable_C")
    (bind _asbp_placeable (cast `/Game/Placeables/BP_Placeable` _array_element))
    (if (not (`/Game/Placeables/BP_Placeable.IsOnFire?` _asbp_placeable))
      (`/Game/Placeables/BP_Placeable.Burn` _asbp_placeable))))