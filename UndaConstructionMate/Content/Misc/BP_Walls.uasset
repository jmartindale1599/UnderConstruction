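; BP_Walls is a wall actor that changes colour when a BP_P_PBrush overlaps one of its two box triggers.
; Box tints the Back mesh with the brush's ColorGive value, while Box1 always turns the Front mesh black.
; Each overlap creates a new dynamic instance of M_BaseChange on the mesh and sets its Color parameter.
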(event `self.Box.OnComponentBeginOverlap`
  (params (OverlappedComponent :type "PrimitiveComponent Object Reference") (OtherActor :type "Actor Object Reference") (OtherComp :type "PrimitiveComponent Object Reference") (OtherBodyIndex :type Integer) (bFromSweep :type Boolean) (SweepResult :type "HitResult Structure (by ref)"))
  (bind _asbp_p_pbrush (cast `/Game/Placeables/BP_P_PBrush` OtherActor))
  (bind _returnvalue (`PrimitiveComponent.CreateDynamicMaterialInstance` (`self.back`) 0 "/Game/Materials/M_BaseChange.M_BaseChange" "None"))
  (`MaterialInstanceDynamic.SetVectorParameterValue` _returnvalue "Color" (`KismetMathLibrary.Conv_ColorToLinearColor` (`/Game/Placeables/BP_P_PBrush.ColorGive` _asbp_p_pbrush))))

(event `self.Box1.OnComponentBeginOverlap`
  (params (OverlappedComponent :type "PrimitiveComponent Object Reference") (OtherActor :type "Actor Object Reference") (OtherComp :type "PrimitiveComponent Object Reference") (OtherBodyIndex :type Integer) (bFromSweep :type Boolean) (SweepResult :type "HitResult Structure (by ref)"))
  (cast `/Game/Placeables/BP_P_PBrush` OtherActor)
  (bind _returnvalue (`PrimitiveComponent.CreateDynamicMaterialInstance` (`self.front`) 0 "/Game/Materials/M_BaseChange.M_BaseChange" "None"))
  (`MaterialInstanceDynamic.SetVectorParameterValue` :`self` _returnvalue :`ParameterName` "Color"))

(fn `UserConstructionScript`)