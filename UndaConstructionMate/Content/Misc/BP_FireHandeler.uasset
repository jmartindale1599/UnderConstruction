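; BP_FireHandeler drives the game's fire spreading across placeable objects.
; StartFireGame caches every BP_Placeable in the level and starts a looping timer for the fire check.
; Each check scans the list, dropping invalid entries until it finds a burning one, then calls Burn on a random entry whether or not one was found.
; An empty list at the start of a check prints "Game Ogre" instead.
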(event `StartFireGame`
  (bind _outactors (`GameplayStatics.GetAllActorsOfClass` "/Game/Placeables/BP_Placeable.BP_Placeable_C"))
  (set `self.FirePeople` _outactors)
  (`KismetSystemLibrary.K2_SetTimerDelegate` (delegate `Any on Fire?`) 5.0 true))

(event `Any on Fire?`
  (bind _firepeople (`self.FirePeople`))
  (if (`KismetArrayLibrary.Array_IsEmpty` (`self.FirePeople`))
    (`KismetSystemLibrary.PrintString` "Game Ogre" true true (struct :`G` 0.66 :`B` 1.0 :`A` 1.0) 12.0)
    (else
      (for (_array_element _array_index) _firepeople
        (`/Engine/EditorBlueprintResources/StandardMacros.IsValid` _array_element
          (:`Is Valid`
            (if (`/Game/Placeables/BP_Placeable.IsOnFire?` _array_element)
              (break)))
          (:`Is Not Valid`
            (`KismetArrayLibrary.Array_Remove` _firepeople _array_index))))
      (`/Game/Placeables/BP_Placeable.Burn` (`KismetArrayLibrary.Array_Random` _firepeople)))))

(fn `UserConstructionScript`)