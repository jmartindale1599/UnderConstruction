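; Grabbable spray bottle that puts out burning BP_Placeable actors with limited water shots.
; Grabbing enables input and adds the mapping context for the holding hand; dropping reverses this.
; Shooting line-traces from the arrow, clears IsOnFire on a hit placeable and spends a shot; only the right-hand path also hides active fire particles.
; The bottle's material reflects remaining shots, and overlapping a BP_Sink with the capsule refills it.
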(event `self.GrabComponent.OnGrabbed`
  ;[0.02745 0.02745 0.02745] What We do when grabbed or dropped
  (`self.EnableInput` (`GameplayStatics.GetPlayerController` 0))
  (`EnhancedInputSubsystemInterface.AddMappingContext` (pcsubsystem `EnhancedInputLocalPlayerSubsystem` (`GameplayStatics.GetPlayerController` 0)) (select `bool` (`|EnumEquality` (`/Game/VRTemplate/Blueprints/GrabComponent.GetHeldByHand` (`self.GrabComponent`)) "Right") :`false` "/Game/VRTemplate/Input/IMC_Weapon_Left.IMC_Weapon_Left" :`true` "/Game/VRTemplate/Input/IMC_Weapon_Right.IMC_Weapon_Right" :!type "InputMappingContext Object Reference") 1 (struct)))

(event `self.GrabComponent.OnDropped`
  ;[0.02745 0.02745 0.02745] What We do when grabbed or dropped
  (`self.DisableInput` (`GameplayStatics.GetPlayerController` 0))
  (`EnhancedInputSubsystemInterface.RemoveMappingContext` (pcsubsystem `EnhancedInputLocalPlayerSubsystem` (`GameplayStatics.GetPlayerController` 0)) (select `bool` (`|EnumEquality` (`/Game/VRTemplate/Blueprints/GrabComponent.GetHeldByHand` (`self.GrabComponent`)) "Right") :`false` "/Game/VRTemplate/Input/IMC_Weapon_Left.IMC_Weapon_Left" :`true` "/Game/VRTemplate/Input/IMC_Weapon_Right.IMC_Weapon_Right" :!type "InputMappingContext Object Reference") (struct)))

(event `self.ReceiveBeginPlay`
  (`PrimitiveComponent.SetMaterial` (`self.spray_bottle`) 0 "/Game/Materials/WaterStages/M_WaterFull.M_WaterFull"))

(event `EnhancedInput|/Game/VRTemplate/Input/Actions/IA_Shoot_Left`
  (params (ActionValue :type Boolean) (ElapsedSeconds :type "Float (double-precision)") (TriggeredSeconds :type "Float (double-precision)") (InputAction :type "InputAction Object Reference" :default "/Game/VRTemplate/Input/Actions/IA_Shoot_Left.IA_Shoot_Left"))
  (bind _arrow (`self.Arrow`))
  (bind _shotstoshoot (`self.ShotsToShoot`))
  (:`Started`
    (if (`|EnumEquality` (`/Game/VRTemplate/Blueprints/GrabComponent.GetHeldByHand` (`self.GrabComponent`)) "Left")
      (bind _outhit (`KismetSystemLibrary.LineTraceSingleForObjects` :`Start` (`SceneComponent.K2_GetComponentLocation` _arrow) :`End` (* (`SceneComponent.GetForwardVector` _arrow) 200000.0) :`ObjectTypes` (`|MakeArray` "ObjectTypeQuery2" "ObjectTypeQuery1" :!type "EObjectTypeQuery Enum") :`DrawDebugType` "ForDuration" :`TraceColor` (struct :`G` 0.715483 :`B` 1.0 :`A` 1.0) :`TraceHitColor` (struct :`G` 0.417661 :`B` 1.0 :`A` 1.0)))
      (bind _asbp_placeable (cast `/Game/Placeables/BP_Placeable` (`.HitActor` (`GameplayStatics.BreakHitResult` _outhit)))
        (:`then`
          (if (> _shotstoshoot 0)
            (set `/Game/Placeables/BP_Placeable.IsOnFire?` false _asbp_placeable)
            (bind _result (`/Engine/EditorBlueprintResources/StandardMacros.DecrementInt` _shotstoshoot)
              (:`  `
                (set `self.ShotsToShoot` _result)
                (`self.UpdateWaerDisp`)))
            (else
              (`KismetSystemLibrary.PrintString` "Out Of Waer" :!label _label))))
        (:`CastFailed`
          (`KismetSystemLibrary.PrintString` "Cant Shoot Here" :!label _label_2))))))

(event `EnhancedInput|/Game/VRTemplate/Input/Actions/IA_Shoot_Right`
  (params (ActionValue :type Boolean) (ElapsedSeconds :type "Float (double-precision)") (TriggeredSeconds :type "Float (double-precision)") (InputAction :type "InputAction Object Reference" :default "/Game/VRTemplate/Input/Actions/IA_Shoot_Right.IA_Shoot_Right"))
  (bind _arrow (`self.Arrow`))
  (bind _shotstoshoot (`self.ShotsToShoot`))
  (:`Started`
    (if (`|EnumEquality` (`/Game/VRTemplate/Blueprints/GrabComponent.GetHeldByHand` (`self.GrabComponent`)) "Right")
      (bind _outhit (`KismetSystemLibrary.LineTraceSingleForObjects` :`Start` (`SceneComponent.K2_GetComponentLocation` _arrow) :`End` (* (`SceneComponent.GetForwardVector` _arrow) 200000.0) :`ObjectTypes` (`|MakeArray` "ObjectTypeQuery2" "ObjectTypeQuery1" :!type "EObjectTypeQuery Enum") :`DrawDebugType` "ForDuration" :`TraceColor` (struct :`G` 0.715483 :`B` 1.0 :`A` 1.0) :`TraceHitColor` (struct :`G` 0.417661 :`B` 1.0 :`A` 1.0)))
      (bind _asbp_placeable (cast `/Game/Placeables/BP_Placeable` (`.HitActor` (`GameplayStatics.BreakHitResult` _outhit)))
        (:`then`
          (if (> _shotstoshoot 0)
            (set `/Game/Placeables/BP_Placeable.IsOnFire?` false _asbp_placeable)
            (bind _particle_system (`/Game/Placeables/BP_Placeable.Particle System` _asbp_placeable))
            (if (`ActorComponent.IsActive` _particle_system)
              (`SceneComponent.SetVisibility` _particle_system false false))
            (bind _result (`/Engine/EditorBlueprintResources/StandardMacros.DecrementInt` _shotstoshoot)
              (:`  `
                (set `self.ShotsToShoot` _result)
                (`self.UpdateWaerDisp`)))
            (else
              (goto _label))))
        (:`CastFailed`
          (goto _label_2))))))

(event `UpdateWaerDisp`
  (bind _spray_bottle (`self.spray_bottle`))
  (switch `int` (`self.ShotsToShoot`)
    (:`Default`
      (`PrimitiveComponent.SetMaterial` _spray_bottle 0 "/Game/Materials/WaterStages/M_WaterEmpty.M_WaterEmpty" :!label _label_3))
    (:`0`
      (goto _label_3))
    (:`1`
      (`PrimitiveComponent.SetMaterial` _spray_bottle 0 "/Game/Materials/WaterStages/M_WaterMid.M_WaterMid"))
    (:`2`
      (`PrimitiveComponent.SetMaterial` _spray_bottle 0 "/Game/Materials/WaterStages/M_WaterLow.M_WaterLow"))
    (:`3`
      (`PrimitiveComponent.SetMaterial` _spray_bottle 0 "/Game/Materials/WaterStages/M_WaterFull.M_WaterFull"))))

(event `self.Capsule.OnComponentBeginOverlap`
  (params (OverlappedComponent :type "PrimitiveComponent Object Reference") (OtherActor :type "Actor Object Reference") (OtherComp :type "PrimitiveComponent Object Reference") (OtherBodyIndex :type Integer) (bFromSweep :type Boolean) (SweepResult :type "HitResult Structure (by ref)"))
  (cast `/Game/Misc/BP_Sink` OtherActor)
  (set `self.ShotsToShoot` 3)
  (`self.UpdateWaerDisp`))

(fn `UserConstructionScript`)