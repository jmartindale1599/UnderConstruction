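; VR placeable building actor that the player grabs, aims with a hologram preview and teleports into place, and that can burn down.
; Grabbing shows the preview and adds the holding hand's weapon input context.
; Tick moves the preview via hand line traces against WorldStatic; the shoot input teleports the actor to the hit, yawed to the headset.
; Burn notifies BPBurnable and starts a looping timer that drains health until destruction.
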(event `on FIre`
  (if (`self.IsOnFire?`)
    (bind _output_get (set `self.Building Health` (- (`self.Building Health`) 2.0)))
    (if (<= _output_get 0.0)
      (`self.destroySelf`))))

(event `Burn`
  (set `self.IsOnFire?` true)
  (`/Game/Misc/BP_Burnable.Set OnFire` (`self.BP_Burnable`) self)
  (`KismetSystemLibrary.K2_SetTimerDelegate` (delegate `on FIre`) 5.0 true))

(event `destroySelf`
  (`self.K2_DestroyActor`))

(event `EnhancedInput|/Game/VRTemplate/Input/Actions/IA_Shoot_Left`
  (params (ActionValue :type Boolean) (ElapsedSeconds :type "Float (double-precision)") (TriggeredSeconds :type "Float (double-precision)") (InputAction :type "InputAction Object Reference" :default "/Game/VRTemplate/Input/Actions/IA_Shoot_Left.IA_Shoot_Left"))
  ;[0.02745 0.02745 0.02745] Bascially how we "place" objects
  (:`Started`
    (if (`|EnumEquality` (`/Game/VRTemplate/Blueprints/GrabComponent.GetHeldByHand` (`self.GrabComponent`)) "Left")
      (bind _returnvalue (`GameplayStatics.GetActorOfClass` "/Game/VRTemplate/Blueprints/VRPawn.VRPawn_C"))
      (bind _lefthandforward (`/Game/VRTemplate/Blueprints/VRPawn.LeftHandForward` _returnvalue))
      (bind _outhit (`KismetSystemLibrary.LineTraceSingleForObjects` :`Start` (`SceneComponent.K2_GetComponentLocation` _lefthandforward) :`End` (* (`SceneComponent.GetForwardVector` _lefthandforward) 200000.0) :`ObjectTypes` (`|MakeArray` "ObjectTypeQuery1" :!type "EObjectTypeQuery Enum") :`DrawDebugType` "ForOneFrame"))
      (`EnhancedInputSubsystemInterface.RemoveMappingContext` (pcsubsystem `EnhancedInputLocalPlayerSubsystem` (`GameplayStatics.GetPlayerController` 0)) (select `bool` (`|EnumEquality` (`/Game/VRTemplate/Blueprints/GrabComponent.GetHeldByHand` (`self.GrabComponent`)) "Right") :`false` "/Game/VRTemplate/Input/IMC_Weapon_Left.IMC_Weapon_Left" :`true` "/Game/VRTemplate/Input/IMC_Weapon_Right.IMC_Weapon_Right" :!type "InputMappingContext Object Reference") (struct))
      (bind (_returnvalue_roll _returnvalue_pitch _returnvalue_yaw) (`KismetMathLibrary.BreakRotator` (`SceneComponent.K2_GetComponentRotation` (`/Game/VRTemplate/Blueprints/VRPawn.HeadMountedDisplayMesh` _returnvalue))))
      (`self.K2_TeleportTo` (`.ImpactPoint` (`GameplayStatics.BreakHitResult` _outhit)) (`KismetMathLibrary.MakeRotator` 0.0 0.0 _returnvalue_yaw)))))

(event `EnhancedInput|/Game/VRTemplate/Input/Actions/IA_Shoot_Right`
  (params (ActionValue :type Boolean) (ElapsedSeconds :type "Float (double-precision)") (TriggeredSeconds :type "Float (double-precision)") (InputAction :type "InputAction Object Reference" :default "/Game/VRTemplate/Input/Actions/IA_Shoot_Right.IA_Shoot_Right"))
  ;[0.02745 0.02745 0.02745] Bascially how we "place" objects
  (:`Started`
    (if (`|EnumEquality` (`/Game/VRTemplate/Blueprints/GrabComponent.GetHeldByHand` (`self.GrabComponent`)) "Right")
      (bind _returnvalue (`GameplayStatics.GetActorOfClass` "/Game/VRTemplate/Blueprints/VRPawn.VRPawn_C"))
      (bind _righthandforward (`/Game/VRTemplate/Blueprints/VRPawn.RightHandForward` _returnvalue))
      (bind _outhit (`KismetSystemLibrary.LineTraceSingleForObjects` :`Start` (`SceneComponent.K2_GetComponentLocation` _righthandforward) :`End` (* (`SceneComponent.GetForwardVector` _righthandforward) 20000.0) :`ObjectTypes` (`|MakeArray` "ObjectTypeQuery1" :!type "EObjectTypeQuery Enum") :`DrawDebugType` "ForOneFrame"))
      (`EnhancedInputSubsystemInterface.RemoveMappingContext` (pcsubsystem `EnhancedInputLocalPlayerSubsystem` (`GameplayStatics.GetPlayerController` 0)) (select `bool` (`|EnumEquality` (`/Game/VRTemplate/Blueprints/GrabComponent.GetHeldByHand` (`self.GrabComponent`)) "Right") :`false` "/Game/VRTemplate/Input/IMC_Weapon_Left.IMC_Weapon_Left" :`true` "/Game/VRTemplate/Input/IMC_Weapon_Right.IMC_Weapon_Right" :!type "InputMappingContext Object Reference") (struct))
      (bind (_returnvalue_roll _returnvalue_pitch _returnvalue_yaw) (`KismetMathLibrary.BreakRotator` (`SceneComponent.K2_GetComponentRotation` (`/Game/VRTemplate/Blueprints/VRPawn.HeadMountedDisplayMesh` _returnvalue))))
      (`self.K2_TeleportTo` (`.ImpactPoint` (`GameplayStatics.BreakHitResult` _outhit)) (`KismetMathLibrary.MakeRotator` 0.0 0.0 _returnvalue_yaw)))))

(event `self.GrabComponent.OnGrabbed`
  ;[0.02745 0.02745 0.02745] What We do when grabbed or dropped
  (`SceneComponent.SetVisibility` (`self.DisplayPrevMesh`) true false)
  (`self.EnableInput` (`GameplayStatics.GetPlayerController` 0))
  (`EnhancedInputSubsystemInterface.AddMappingContext` (pcsubsystem `EnhancedInputLocalPlayerSubsystem` (`GameplayStatics.GetPlayerController` 0)) (select `bool` (`|EnumEquality` (`/Game/VRTemplate/Blueprints/GrabComponent.GetHeldByHand` (`self.GrabComponent`)) "Right") :`false` "/Game/VRTemplate/Input/IMC_Weapon_Left.IMC_Weapon_Left" :`true` "/Game/VRTemplate/Input/IMC_Weapon_Right.IMC_Weapon_Right" :!type "InputMappingContext Object Reference") 1 (struct)))

(event `self.GrabComponent.OnDropped`
  ;[0.02745 0.02745 0.02745] What We do when grabbed or dropped
  (`SceneComponent.SetVisibility` (`self.DisplayPrevMesh`) false false)
  (`self.DisableInput` (`GameplayStatics.GetPlayerController` 0))
  (`EnhancedInputSubsystemInterface.RemoveMappingContext` (pcsubsystem `EnhancedInputLocalPlayerSubsystem` (`GameplayStatics.GetPlayerController` 0)) (select `bool` (`|EnumEquality` (`/Game/VRTemplate/Blueprints/GrabComponent.GetHeldByHand` (`self.GrabComponent`)) "Right") :`false` "/Game/VRTemplate/Input/IMC_Weapon_Left.IMC_Weapon_Left" :`true` "/Game/VRTemplate/Input/IMC_Weapon_Right.IMC_Weapon_Right" :!type "InputMappingContext Object Reference") (struct)))

(event `self.ReceiveTick`
  (params (DeltaSeconds :type "Float (single-precision)"))
  (bind _displayprevmesh (`self.DisplayPrevMesh`))
  (bind _returnvalue (`/Game/VRTemplate/Blueprints/GrabComponent.GetHeldByHand` (`self.GrabComponent`)))
  (bind _returnvalue_2 (`|EnumEquality` _returnvalue "Left"))
  ;[0.02745 0.02745 0.02745] Rough Display For where place when something is grabbed
  (if (`/Game/VRTemplate/Blueprints/GrabComponent.bIsHeld` (`self.GrabComponent`))
    (bind _returnvalue_3 (`GameplayStatics.GetActorOfClass` "/Game/VRTemplate/Blueprints/VRPawn.VRPawn_C"))
    (if (and _returnvalue_2 (`|EnumEquality` _returnvalue "Right"))
      (`|ExecutionSequence`
        (:`then_0`
          (bind _lefthandforward (`/Game/VRTemplate/Blueprints/VRPawn.LeftHandForward` _returnvalue_3))
          (bind _outhit (`KismetSystemLibrary.LineTraceSingleForObjects` :`Start` (`SceneComponent.K2_GetComponentLocation` _lefthandforward) :`End` (* (`SceneComponent.GetForwardVector` _lefthandforward) 200000.0) :`ObjectTypes` (`|MakeArray` "ObjectTypeQuery1" :!type "EObjectTypeQuery Enum") :`DrawDebugType` "ForOneFrame"))
          (bind (_returnvalue_roll _returnvalue_pitch _returnvalue_yaw) (`KismetMathLibrary.BreakRotator` (`SceneComponent.K2_GetComponentRotation` (`/Game/VRTemplate/Blueprints/VRPawn.HeadMountedDisplayMesh` _returnvalue_3))))
          (`SceneComponent.K2_SetWorldTransform` _displayprevmesh (`KismetMathLibrary.MakeTransform` (`.ImpactNormal` (`GameplayStatics.BreakHitResult` _outhit)) (`KismetMathLibrary.MakeRotator` 0.0 0.0 _returnvalue_yaw)) false true))
        (:`then_1`
          (bind _righthandforward (`/Game/VRTemplate/Blueprints/VRPawn.RightHandForward` _returnvalue_3))
          (bind _outhit_2 (`KismetSystemLibrary.LineTraceSingleForObjects` :`Start` (`SceneComponent.K2_GetComponentLocation` _righthandforward) :`End` (* (`SceneComponent.GetForwardVector` _righthandforward) 200000.0) :`ObjectTypes` (`|MakeArray` "ObjectTypeQuery1" :!type "EObjectTypeQuery Enum") :`DrawDebugType` "ForOneFrame"))
          (`SceneComponent.K2_SetWorldTransform` _displayprevmesh (`KismetMathLibrary.MakeTransform` (`.ImpactPoint` (`GameplayStatics.BreakHitResult` _outhit_2)) (`KismetMathLibrary.MakeRotator` 0.0 0.0 _returnvalue_yaw)) false true)))
      (elif _returnvalue_2
        (bind _lefthandforward_2 (`/Game/VRTemplate/Blueprints/VRPawn.LeftHandForward` _returnvalue_3))
        (bind _outhit_3 (`KismetSystemLibrary.LineTraceSingleForObjects` :`Start` (`SceneComponent.K2_GetComponentLocation` _lefthandforward_2) :`End` (* (`SceneComponent.GetForwardVector` _lefthandforward_2) 200000.0) :`ObjectTypes` (`|MakeArray` "ObjectTypeQuery1" :!type "EObjectTypeQuery Enum") :`DrawDebugType` "ForOneFrame"))
        (bind (_returnvalue_roll_2 _returnvalue_pitch_2 _returnvalue_yaw_2) (`KismetMathLibrary.BreakRotator` (`SceneComponent.K2_GetComponentRotation` (`/Game/VRTemplate/Blueprints/VRPawn.HeadMountedDisplayMesh` _returnvalue_3))))
        (`SceneComponent.K2_SetWorldTransform` (`self.DisplayPrevMesh`) (`KismetMathLibrary.MakeTransform` (`.ImpactPoint` (`GameplayStatics.BreakHitResult` _outhit_3)) (`KismetMathLibrary.MakeRotator` 0.0 0.0 _returnvalue_yaw_2)) false true)
        (else
          (bind _righthandforward_2 (`/Game/VRTemplate/Blueprints/VRPawn.RightHandForward` _returnvalue_3))
          (bind _outhit_4 (`KismetSystemLibrary.LineTraceSingleForObjects` :`Start` (`SceneComponent.K2_GetComponentLocation` _righthandforward_2) :`End` (* (`SceneComponent.GetForwardVector` _righthandforward_2) 200000.0) :`ObjectTypes` (`|MakeArray` "ObjectTypeQuery1" :!type "EObjectTypeQuery Enum") :`DrawDebugType` "ForOneFrame"))
          (bind (_returnvalue_roll_3 _returnvalue_pitch_3 _returnvalue_yaw_3) (`KismetMathLibrary.BreakRotator` (`SceneComponent.K2_GetComponentRotation` (`/Game/VRTemplate/Blueprints/VRPawn.HeadMountedDisplayMesh` _returnvalue_3))))
          (`SceneComponent.K2_SetWorldTransform` (`self.DisplayPrevMesh`) (`KismetMathLibrary.MakeTransform` (`.ImpactPoint` (`GameplayStatics.BreakHitResult` _outhit_4)) (`KismetMathLibrary.MakeRotator` 0.0 0.0 _returnvalue_yaw_3)) false true))))))

(event `self.ReceiveBeginPlay`
  (bind _returnvalue (`AddComponent|NODE_AddStaticMeshComponent-0` :`RelativeTransform` (`KismetMathLibrary.MakeTransform` (0.0 0.0 0.0))))
  (`PrimitiveComponent.SetCollisionObjectType` _returnvalue "ECC_WorldDynamic")
  (`PrimitiveComponent.SetCollisionEnabled` _returnvalue "NoCollision")
  (bind _output_get (set `self.DisplayPrevMesh` _returnvalue))
  (`SceneComponent.SetVisibility` _output_get false false)
  (`StaticMeshComponent.SetStaticMesh` _output_get (`self.Static Mesh Ref`))
  (for (_ _array_index) (`MeshComponent.GetMaterials` _output_get)
    (`PrimitiveComponent.SetMaterial` _output_get _array_index "/Game/Materials/M_Hologram.M_Hologram")))

(fn `UserConstructionScript`)