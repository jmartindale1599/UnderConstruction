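; BP_Doorknob is a grabbable placeable doorknob that triggers the fire game.
; When its GrabComponent fires OnGrabbed, it plays a fire alarm sound at the actor's location.
; It then looks up the BP_FireHandeler actor in the level and, if valid, calls StartFireGame on it.
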(event `self.GrabComponent.OnGrabbed`
  (`GameplayStatics.PlaySoundAtLocation` "/Game/Audio/fire-alarm-9677.fire-alarm-9677" (`self.K2_GetActorLocation` self) (struct) 1.0 1.0 0.0 null null null null)
  (bind _returnvalue (`GameplayStatics.GetActorOfClass` "/Game/Misc/BP_FireHandeler.BP_FireHandeler_C"))
  (`/Engine/EditorBlueprintResources/StandardMacros.IsValid` _returnvalue
    (:`Is Valid`
      (`/Game/Misc/BP_FireHandeler.StartFireGame` _returnvalue))))

(fn `UserConstructionScript`
  (`parent.UserConstructionScript`))